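; BP_AreaWarningVolume is a play-area boundary that damages the player when a BP_Marine leaves it.
; Exiting sets the marine's OutsideArea flag, deals damage immediately, and starts a looping KillPlayer timer at the SpeedOfKillPlayer interval.
; Re-entering clears the flag and timer.
; KillPlayer always applies OutsideAreaDamage to player character 0, regardless of which marine crossed the boundary.
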(event `self.ReceiveActorBeginOverlap`
  (params (OtherActor :type "Actor Object Reference"))
  ;[1 1 1] Enter
  (bind _asbp_marine (cast `/Game/Blueprints/Pawns/BP_Marine` OtherActor))
  (set `/Game/Blueprints/Pawns/BP_Marine.OutsideArea` false _asbp_marine)
  (`KismetSystemLibrary.K2_ClearTimer` null "KillPlayer"))

(event `self.ReceiveActorEndOverlap`
  (params (OtherActor :type "Actor Object Reference"))
  ;[1 1 1] Leave
  (bind _asbp_marine (cast `/Game/Blueprints/Pawns/BP_Marine` OtherActor))
  (set `/Game/Blueprints/Pawns/BP_Marine.OutsideArea` true _asbp_marine)
  (`self.KillPlayer`)
  (`KismetSystemLibrary.K2_SetTimer` null "KillPlayer" (`self.SpeedOfKillPlayer`) true))

(fn `KillPlayer`
  (`GameplayStatics.ApplyDamage` (`GameplayStatics.GetPlayerCharacter` 0) (`self.OutsideAreaDamage`)))

(fn `UserConstructionScript`)