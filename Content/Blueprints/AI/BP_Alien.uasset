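; BP_Alien is an enemy AI pawn that chases the player and attacks in melee until killed.
; After a start delay it repeatedly calls AIMoveTo on the player, while Tick plays an attack montage when in range, pausing movement until it completes.
; AnyDamage reduces clamped health; at zero the alien disables collision, registers its death with BP_GameMode, increments BP_Marine's kills and destroys itself after a delay.
; DamagePlayer applies hit damage but has no caller here.
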(event `self.ReceiveAnyDamage`
  (params (Damage :type "Float (single-precision)") (DamageType :type "DamageType Object Reference") (InstigatedBy :type "Controller Object Reference") (DamageCauser :type "Actor Object Reference"))
  ;[1 1 1] Damage
  (if (`self.IsAliienAlive`)
    (bind _health (`self.DecreaseHealth` Damage))
    (if (== _health 0.0)
      (`self.KillAI`)
      (bind _asbp_marine (cast `/Game/Blueprints/Pawns/BP_Marine` (`GameplayStatics.GetPlayerCharacter` 0)))
      (`/Game/Blueprints/Pawns/BP_Marine.IncreaseKills` _asbp_marine)
      (`KismetSystemLibrary.Delay` 3.0)
      (`self.K2_DestroyActor`))))

(event `self.ReceiveBeginPlay`
  ;[1 1 1] MOVE TO PLAYER
  (`KismetSystemLibrary.Delay` 5.0)
  (if (`self.IsAliienAlive`) :!label _label
    (`|AIMoveTo` self (0.0 0.0 0.0) (`GameplayStatics.GetPlayerCharacter` 0)
      (:`OnSuccess`
        _)
      (:`OnFail`
        _))
    (`KismetSystemLibrary.Delay` 0.2)
    (goto _label)))

(event `self.ReceiveTick`
  (params (DeltaSeconds :type "Float (single-precision)"))
  ;[1 1 1] ATTACK
  (if (`self.CanAttack`)
    (`self.Deactivate Attack`)
    (`|PlayMontage` (`self.Mesh`) "/Game/Characters/Enemy_Great_Spider/Animations/AM_AlienAttack_01.AM_AlienAttack_01"
      (:`OnCompleted`
        (`self.Activate Attack`)))))

(fn `Activate Attack`
  (`ActorComponent.Activate` (`self.CharacterMovement`) false))

(fn `CanAttack`
  (returns (ReturnValue :type Boolean))
  (return (and (`self.IsWithinAttackRange`) (`self.IsAliienAlive`) (not (`self.IsAttacking`)))))

(fn `Damage Player`
  (if (`self.IsAliienAlive`)
    (`GameplayStatics.ApplyDamage` (`GameplayStatics.GetPlayerCharacter` 0) (`self.DamagePerHit`))))

(fn `Deactivate Attack`
  (`ActorComponent.Deactivate` (`self.CharacterMovement`)))

(fn `DecreaseHealth`
  (params (DamageAmount :type "Float (double-precision)"))
  (returns (Health :type "Float (double-precision)"))
  (bind _output_get (set `self.AlienHealth` (`KismetMathLibrary.FClamp` (- (`self.AlienHealth`) DamageAmount) 0.0 100.0)))
  (return _output_get))

(fn `IsAliienAlive`
  (returns (ReturnValue :type Boolean))
  (return (not (`self.Dead`))))

(fn `IsAttacking`
  (returns (ReturnValue :type Boolean))
  (return (`AnimInstance.Montage_IsPlaying` (`SkeletalMeshComponent.GetAnimInstance` (`self.Mesh`)) "/Game/Characters/Enemy_Great_Spider/Animations/AM_AlienAttack_01.AM_AlienAttack_01")))

(fn `IsWithinAttackRange`
  (returns (ReturnValue :type Boolean))
  (return (< (`self.GetDistanceTo` (`GameplayStatics.GetPlayerCharacter` 0)) (`self.AttackRange`))))

(fn `KillAI`
  (bind _charactermovement (`self.CharacterMovement`))
  (set `self.Dead` true)
  (`MovementComponent.StopMovementImmediately` _charactermovement)
  (`ActorComponent.Deactivate` _charactermovement)
  (`self.SetActorEnableCollision` false)
  (bind _asbp_game_mode (cast `/Game/Blueprints/GameMode/BP_GameMode` (`GameplayStatics.GetGameMode`)))
  (`/Game/Blueprints/GameMode/BP_GameMode.RegisterAlienDeath` _asbp_game_mode self))

(fn `UserConstructionScript`)